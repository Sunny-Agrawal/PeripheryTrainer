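; AR pawn that starts and stops an AR session with play and tests gaze targeting through a camera-origin line trace.
; Each tick it projects eye-tracker gaze from the camera and runs a debug-drawn Visibility trace, leaving the hit unused.
; Without a tracker, holding G substitutes a trace endpoint built from the normalized viewport mouse position, scaled but not offset by camera location.
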(event Custom|PrepareForAR
  (Class|ARBlueprintLibrary|StartARSession "/Game/Assets/AR_SessionConfig.AR_SessionConfig"))

(event Custom|EyeGazeTracking
  (if (Class|EyeTrackerFunctionLibrary|IsEyeTrackerConnected)
    (bind (_outgazedata _returnvalue) (Class|EyeTrackerFunctionLibrary|GetGazeData))
    (if _returnvalue
      (Variables|Default|SetGazeVector (+ (Transformation|GetWorldLocation (Variables|Default|GetCamera)) (* (.gazedirection _outgazedata) 5e+02)))
      (Collision|LineTraceByChannel (Transformation|GetWorldLocation (Variables|Default|GetCamera)) (Variables|Default|GetGazeVector) "TraceTypeQuery1" false 0 "ForOneFrame" :!label _label))
    (elif (Variables|Default|GetControllingGaze)
      (bind _returnvalue_2 (Class|WidgetLayoutLibrary|GetMousePositiononViewport))
      (Variables|Default|SetGazeVector (* (Math|Vector|Normalize (Math|Conversions|ToVector(Vector2D) _returnvalue_2 2e+01)) 5e+02))
      (goto _label))))

(event EventBeginPlay
  (CallFunction|PrepareforAR))

(event Collision|EventActorBeginOverlap
  (params (OtherActor :type Actor%20Object%20Reference)))

(event EventTick
  (params (DeltaSeconds :type Float%20%28single-precision%29))
  (CallFunction|EyeGazeTracking))

(event EventEndPlay
  (params (EndPlayReason :type EEndPlayReason%20Enum :default "Destroyed"))
  (Class|ARBlueprintLibrary|StopARSession))

(event Input|KeyboardEvents|G
  (params (Key :type Key%20Structure :default "None"))
  (:Pressed
    (Variables|Default|SetControllingGaze true))
  (:Released
    (Variables|Default|SetControllingGaze false)))

(fn ConstructionScript)